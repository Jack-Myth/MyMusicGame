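; Player pawn that runs a rhythm game session: spawning notes, routing hole hits, pausing and showing results.
; INITGame loads the selected song's chart and audio, pre-spawns up to 100 RhythmNotes at four holes; SpawnNewRhythmNote streams the rest.
; Tick advances a millisecond clock, zeroed on the first audio playback callback; note times include the saved player offset.
; Typed hits the earliest hittable note in that hole; CheckLast shows full-combo or all-Charming banners.
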(event OnAudioPlaybackPercent(Audio)
  (params (PlayingSoundWave :type Sound%20Wave%20Object%20Reference) (PlaybackPercent :type Float%20%28single-precision%29))
  (Utilities|FlowControl|DoOnce false
    (:Completed
      (Variables|Default|SetCurTime 0.0))))

(event ApplicationWillEnterBackgroundDelegate(ApplicationLifecycle)
  (if (not (Variables|Default|GetIsGamePaused))
    (Variables|Default|SetIsGamePaused true)
    (Development|ExecuteConsoleCommand "ce GamePaused")
    (Game|SetGamePaused true)
    (bind _returnvalue (UserInterface|CreateWidget "/Game/MyMusicGame/Blueprints/UI/PauseUI.PauseUI_C"))
    (UserInterface|Viewport|AddtoViewport _returnvalue 0)))

(event OnAudioFinished(Audio)
  (Actor|Tick|SetActorTickEnabled false)
  (bind _outactors (Actor|GetAllActorsOfClass "/Game/MyMusicGame/Blueprints/RhythmNote.RhythmNote_C"))
  (Actor|DestroyActor _outactors)
  (bind _returnvalue (UserInterface|CreateWidget "/Game/MyMusicGame/Blueprints/UI/ResultUI.ResultUI_C"))
  (UserInterface|Viewport|AddtoViewport _returnvalue 0)
  (Utilities|FlowControl|Delay 2.0)
  (Widget|RemovefromParent (Variables|Default|GetGameUI)))

(event Custom|INITGame
  (params (Hole0 :type Rhythm%20Hole%20Object%20Reference) (Hole1 :type Rhythm%20Hole%20Object%20Reference) (Hole2 :type Rhythm%20Hole%20Object%20Reference) (Hole3 :type Rhythm%20Hole%20Object%20Reference))
  (bind _mygameinstance (Utilities|MYGameInstance))
  (bind _audio (Variables|Default|GetAudio))
  (bind _holecollection (Variables|Default|GetHoleCollection))
  (bind _musicnamef (Variables|/Game/MyMusicGame/Blueprints/GameMode/MYGameInstance.MYGameInstance_C|GetMusicNameF _mygameinstance))
  (bind _musiclevel (Variables|/Game/MyMusicGame/Blueprints/GameMode/MYGameInstance.MYGameInstance_C|GetMusicLevel _mygameinstance))
  (bind _returnvalue (UserInterface|CreateWidget "/Game/MyMusicGame/Blueprints/UI/GameUI.GameUI_C"))
  (bind _output_get (Variables|Default|SetGameUI _returnvalue))
  (UserInterface|Viewport|AddtoViewport _output_get 0)
  (Utilities|ClearStage)
  (Utilities|FlowControl|Sequence
    (:then_0
      (Utilities|Array|Add _holecollection Hole0))
    (:then_1
      (Utilities|Array|Add _holecollection Hole1))
    (:then_2
      (Utilities|Array|Add _holecollection Hole2))
    (:then_3
      (Utilities|Array|Add _holecollection Hole3))
    (:then_4
      (bind _outactors (Actor|GetAllActorsOfClass "/Script/MyMusicGame.FunctionLibrary"))
      (bind _returnvalue_2 (Class|FunctionLibrary|GetMusicAlbumPic (Utilities|Array|Get(acopy) _outactors) _musicnamef))
      (Variables|Default|SetMusicAlbumPic _returnvalue_2)
      (bind _returnvalue_3 (Class|FunctionLibrary|GetMusicName (Utilities|Array|Get(acopy) _outactors) _musicnamef))
      (Variables|Default|SetMusicName _returnvalue_3)
      (bind _returnvalue_4 (Class|FunctionLibrary|GetMusicianName (Utilities|Array|Get(acopy) _outactors) _musicnamef))
      (Variables|Default|SetMusicianName _returnvalue_4)
      (bind _returnvalue_5 (Class|FunctionLibrary|GetMusicRhythmNotes (Utilities|Array|Get(acopy) _outactors) _musicnamef _musiclevel))
      (Variables|Default|SetRhythmCount (Utilities|Array|Length _returnvalue_5))
      (Variables|Default|SetSingleScore (/ 1e+02 (Math|Conversions|ToFloat(Integer) (Utilities|Array|Length _returnvalue_5))))
      (bind _output_get_2 (Variables|Default|SetRhythmD _returnvalue_5))
      (bind _index (Utilities|FlowControl|ForLoopwithBreak 0 99 :!label _label)
        (:LoopBody
          (if (< _index (Utilities|Array|Length _output_get_2))
            (Game|SpawnActorfromClass "/Game/MyMusicGame/Blueprints/RhythmNote.RhythmNote_C" (Math|Transform|MakeTransform "0.000000, 0,-100.000000" "0, 0, 0" "1,1,1.000000") "Undefined" 0 (+ (.Time (Utilities|Struct|BreakRhythmData (Utilities|Array|Get(acopy) _output_get_2 _index))) (Variables|Default|GetRhythmOffset)) (.Position (Utilities|Struct|BreakRhythmData (Utilities|Array|Get(acopy) _output_get_2 _index))) (Utilities|Select :Index (.Type (Utilities|Struct|BreakRhythmData (Utilities|Array|Get(acopy) _output_get_2 _index))) :Option%200 "NewEnumerator0" :Option%201 "NewEnumerator1") (Transformation|GetActorLocation (Utilities|Array|Get(acopy) (Variables|Default|GetHoleCollection) (.Position (Utilities|Struct|BreakRhythmData (Utilities|Array|Get(acopy) _output_get_2 _index))))) (Variables|/Game/MyMusicGame/Blueprints/GameMode/MYGameInstance.MYGameInstance_C|GetMusicSpeed _mygameinstance) self)
            (Variables|Default|SetRhythmIndex _index)
            (else
              (goto _label Break))))
        (:Completed
          (bind _returnvalue_6 (Class|FunctionLibrary|GetMusicFilePath (Utilities|Array|Get(acopy) _outactors) _musicnamef _musiclevel))
          (bind _returnvalue_7 (Class|FunctionLibrary|GetSoundWavefromFile (Utilities|Array|Get(acopy) _outactors) _returnvalue_6))
          (Audio|Components|Audio|SetSound _audio _returnvalue_7)
          (Audio|Components|Audio|Stop _audio)
          (Audio|Components|Audio|Play _audio 0.0)
          (Actor|Tick|SetActorTickEnabled true)
          (Utilities|FlowControl|DoOnce false) ; enters at Reset
        )))))

(event Custom|SpawnNewRhythmNote
  (bind _rhythmd (Variables|Default|GetRhythmD))
  (if (< (+ (Variables|Default|GetRhythmIndex) 1) (Utilities|Array|Length _rhythmd))
    (Game|SpawnActorfromClass "/Game/MyMusicGame/Blueprints/RhythmNote.RhythmNote_C" (Math|Transform|MakeTransform "0.000000, 0,-100.000000" "0, 0, 0" "1,1,1.000000") "Undefined" 0 (+ (.Time (Utilities|Struct|BreakRhythmData (Utilities|Array|Get(acopy) _rhythmd (+ (Variables|Default|GetRhythmIndex) 1)))) (Variables|Default|GetRhythmOffset)) (.Position (Utilities|Struct|BreakRhythmData (Utilities|Array|Get(acopy) _rhythmd (+ (Variables|Default|GetRhythmIndex) 1)))) (Utilities|Select :Index (.Type (Utilities|Struct|BreakRhythmData (Utilities|Array|Get(acopy) _rhythmd (+ (Variables|Default|GetRhythmIndex) 1)))) :Option%200 "NewEnumerator0" :Option%201 "NewEnumerator1") (Transformation|GetActorLocation (Utilities|Array|Get(acopy) (Variables|Default|GetHoleCollection) (.Position (Utilities|Struct|BreakRhythmData (Utilities|Array|Get(acopy) _rhythmd (+ (Variables|Default|GetRhythmIndex) 1)))))) (Variables|/Game/MyMusicGame/Blueprints/GameMode/MYGameInstance.MYGameInstance_C|GetMusicSpeed (Utilities|MYGameInstance)) self)
    (Variables|Default|SetRhythmIndex (+ (Variables|Default|GetRhythmIndex) 1))))

(event Custom|Typed
  (params (TypedHole :type Rhythm%20Hole%20Object%20Reference))
  (Variables|Default|SetTmpMostMin 0)
  (bind _outactors (Actor|GetAllActorsOfClass "/Game/MyMusicGame/Blueprints/RhythmNote.RhythmNote_C"))
  (for _array_element _outactors
    (if (== (Variables|/Game/MyMusicGame/Blueprints/RhythmNote.RhythmNote_C|GetPosition _array_element) (Utilities|Array|FindItem (Variables|Default|GetHoleCollection) TypedHole))
      (bind _canbetyped (Default|CanbeTyped _array_element))
      (if _canbetyped
        (if (== (Variables|Default|GetTmpMostMin) 0)
          (Variables|Default|SetTmpMostMin _array_element :!label _label)
          (elif (< (Variables|/Game/MyMusicGame/Blueprints/RhythmNote.RhythmNote_C|GetTime _array_element) (Variables|/Game/MyMusicGame/Blueprints/RhythmNote.RhythmNote_C|GetTime (Variables|Default|GetTmpMostMin)))
            (goto _label))))))
  (Utilities|IsValid (Variables|Default|GetTmpMostMin)
    (:Is%20Valid
      (Default|EventSuccessfulTyped (Variables|Default|GetTmpMostMin)))))

(event Custom|CheckLast
  (bind _rhythmcount (Variables|Default|GetRhythmCount))
  (bind _outactors (Actor|GetAllActorsOfClass "/Game/MyMusicGame/Blueprints/RhythmNote.RhythmNote_C"))
  (if (<= (Utilities|Array|Length _outactors) 1)
    (if (== (Variables|Default|GetCharmingCount) _rhythmcount)
      (bind _returnvalue (UserInterface|CreateWidget "/Game/MyMusicGame/Blueprints/UI/FCAC_InGame.FCAC_InGame_C"))
      (Default|Init _returnvalue true)
      (UserInterface|Viewport|AddtoViewport _returnvalue 0)
      (elif (== (Variables|Default|GetMaxCombo) _rhythmcount)
        (bind _returnvalue_2 (UserInterface|CreateWidget "/Game/MyMusicGame/Blueprints/UI/FCAC_InGame.FCAC_InGame_C"))
        (Default|Init _returnvalue_2 false)
        (UserInterface|Viewport|AddtoViewport _returnvalue_2 0)))))

(event Custom|SetHolePressState
  (params (PressingHole :type Rhythm%20Hole%20Object%20Reference) (IsPressing :type Boolean))
  (Utilities|Array|SetArrayElem (Variables|Default|GetHolePressing) (Utilities|Array|FindItem (Variables|Default|GetHoleCollection) PressingHole) IsPressing))

(event Custom|TypeCharming
  (Default|ShowCharming (Variables|Default|GetGameUI))
  (Math|Integer|IncrementInt (Variables|Default|GetCharmingCount)))

(event EventBeginPlay
  (bind _returnvalue (SaveGame|LoadGamefromSlot "PlayerInfo"))
  (bind _asplayer_info (Utilities|Casting|CastToPlayerInfo _returnvalue))
  (Variables|Default|SetRhythmOffset (Math|Float|Truncate (* 1000 (Variables|/Game/MyMusicGame/Blueprints/GameMode/PlayerInfo.PlayerInfo_C|GetOffset _asplayer_info))))
  (Development|ExecuteConsoleCommand "ce InitLevelInfo"))

(event EventTick
  (params (DeltaSeconds :type Float%20%28single-precision%29))
  (bind _output_get (Variables|Default|SetCurTime (+ (* 1000 DeltaSeconds) (Variables|Default|GetCurTime))))
  (Variables|Default|SetCurPercentage (/ _output_get (* 1000 (Variables|/Script/Engine.SoundBase|GetDuration (Variables|/Script/Engine.AudioComponent|GetSound (Variables|Default|GetAudio))))))
  (Development|PrintString (Utilities|String|ToString(Float) (Variables|Default|GetCurTime)) true true "(R=0.000000,G=0.660000,B=1.000000,A=1.000000)" 0.0))

(event Input|ActionEvents|InputActionBack
  (params (Key :type Key%20Structure :default "AnyKey"))
  (:Pressed
    (if (not (Variables|Default|GetIsGamePaused))
      (Variables|Default|SetIsGamePaused true)
      (Development|ExecuteConsoleCommand "ce GamePaused")
      (Game|SetGamePaused true)
      (bind _returnvalue (UserInterface|CreateWidget "/Game/MyMusicGame/Blueprints/UI/PauseUI.PauseUI_C"))
      (UserInterface|Viewport|AddtoViewport _returnvalue 0))))

(fn ConstructionScript)
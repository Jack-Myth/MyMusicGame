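; ClickableBox is a touch-clickable, textured world object made of a collision Box and a display Plane.
; The construction script creates a dynamic material instance for the Plane and feeds its texture into the Pic parameter.
; SetClickBoxSize maps a 2D size to the Box's X and Z extents.
; Ending a touch on the Box calls CallEventClick only when no top-level user widgets exist, so open UI blocks clicks.
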(event OnInputTouchEnd(Box)
  (params (FingerIndex :type ETouchIndex%20Enum :default "Touch1") (TouchedComponent :type Primitive%20Component%20Object%20Reference))
  (bind _foundwidgets (Widget|GetAllWidgetsOfClass "/Script/UMG.UserWidget" true))
  (if (== (Utilities|Array|Length _foundwidgets) 0)
    (Default|CallEventClick)))

(event Custom|SetClickBoxSize
  (params (Size :type Vector%202D%20Structure))
  (Components|Box|SetBoxExtent (Variables|Default|GetBox) (Math|Vector|MakeVector (.x Size) 0.0 (.y Size)) true))

(fn ConstructionScript
  (bind _returnvalue (Rendering|Material|CreateDynamicMaterialInstance "/Game/MyMusicGame/Materials/ClickableBoxMaterial.ClickableBoxMaterial" :!class /Script/Engine.KismetMaterialLibrary))
  (Rendering|Material|SetTextureParameterValue _returnvalue "Pic" (Variables|Default|GetTexture2d))
  (Rendering|Material|SetMaterial (Variables|Default|GetPlane) 0 _returnvalue))
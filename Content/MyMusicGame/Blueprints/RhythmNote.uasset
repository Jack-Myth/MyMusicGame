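; Rhythm note actor that slides along X according to its hit time versus the player's song clock.
; Timing windows grade hits as charming or normal; a successful hit updates score and combo, triggers effects and requests the next note.
; Pressed-type notes poll on a looping timer and auto-hit while their hole is held.
; Notes left too late break the combo, fade particle alpha via timeline and destroy themselves.
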(event Custom|EventSuccessfulTyped
  (bind _playerref (Variables|Default|GetPlayerREF))
  (bind _playerref_2 (Variables|Default|GetPlayerREF))
  (bind _playerref_3 (Variables|Default|GetPlayerREF))
  (bind _singlescore (Variables|/Game/MyMusicGame/Blueprints/GameMode/GamePawn.GamePawn_C|GetSingleScore _playerref))
  (bind _combo (Variables|/Game/MyMusicGame/Blueprints/GameMode/GamePawn.GamePawn_C|GetCombo _playerref_2))
  ;[1 1 1] Rhythm Has Been Actived
  (Effects|SpawnEmitteratLocation (Utilities|Select :Index (Variables|Default|GetType) :NewEnumerator0 "/Game/MyMusicGame/Effects/FX_Stars_Burst_Music.FX_Stars_Burst_Music" :NewEnumerator1 "/Game/MyMusicGame/Effects/FX_Stars_Burst_Music_Small.FX_Stars_Burst_Music_Small") (Transformation|GetActorLocation))
  (bind _ischarming (CallFunction|CanbeTyped))
  (Default|TypeEffect (Utilities|Array|Get(acopy) (Variables|/Game/MyMusicGame/Blueprints/GameMode/GamePawn.GamePawn_C|GetHoleCollection (Variables|Default|GetPlayerREF)) (Variables|Default|GetPosition)) _ischarming)
  (if _ischarming
    (Variables|/Game/MyMusicGame/Blueprints/GameMode/GamePawn.GamePawn_C|SetScore _playerref (+ (Variables|/Game/MyMusicGame/Blueprints/GameMode/GamePawn.GamePawn_C|GetScore _playerref) _singlescore))
    (Default|TypeCharming _playerref_2)
    (else
      (Variables|/Game/MyMusicGame/Blueprints/GameMode/GamePawn.GamePawn_C|SetScore _playerref (+ (Variables|/Game/MyMusicGame/Blueprints/GameMode/GamePawn.GamePawn_C|GetScore _playerref) (/ _singlescore 2.0)))))
  (Math|Integer|IncrementInt _combo
    (:%20%20
      (if (< (Variables|/Game/MyMusicGame/Blueprints/GameMode/GamePawn.GamePawn_C|GetMaxCombo _playerref_2) _combo)
        (Variables|/Game/MyMusicGame/Blueprints/GameMode/GamePawn.GamePawn_C|SetMaxCombo _playerref_2 _combo))
      (Default|SpawnNewRhythmNote _playerref_3)
      (Default|CheckLast _playerref_3)
      (Actor|DestroyActor))))

(event Custom|FadeOut
  (bind _playerref (Variables|Default|GetPlayerREF))
  (Actor|Tick|SetActorTickEnabled false)
  (Variables|/Game/MyMusicGame/Blueprints/GameMode/GamePawn.GamePawn_C|SetCombo _playerref 0)
  (Default|SpawnNewRhythmNote _playerref)
  (bind _新建轨迹_0 (Timeline|时间轴_0 Play)
    (:Update
      (Effects|Components|ParticleSystem|SetFloatParameter (Variables|Default|GetParticleSystem) "Alpha" _新建轨迹_0))
    (:Finished
      (Actor|DestroyActor))))

(event EventTick
  (params (DeltaSeconds :type Float%20%28single-precision%29))
  (bind _playerref (Variables|Default|GetPlayerREF))
  (bind _vectorposition (Variables|Default|GetVectorPosition))
  (bind _time (Variables|Default|GetTime))
  (bind _returnvalue (Math|Conversions|ToFloat(Integer) _time))
  (bind _curtime (Variables|/Game/MyMusicGame/Blueprints/GameMode/GamePawn.GamePawn_C|GetCurTime _playerref))
  (bind _returnvalue_2 (- _returnvalue _curtime))
  (bind _returnvalue_3 (/ _returnvalue_2 1e+01))
  ;[1 1 1] Position Offset To Fit Time
  (Transformation|SetActorLocation (Math|Vector|MakeVector (select (>= _returnvalue_2 0.0) (* _returnvalue_3 (Variables|Default|GetSpeed)) _returnvalue_3) (.y _vectorposition) (+ (.z _vectorposition) 1e+02)) false false)
  (if (<= _returnvalue_2 -501.0)
    (CallFunction|FadeOut)))

(event EventBeginPlay
  (bind _type (Variables|Default|GetType))
  ;[1 1 1] Init Timer For Rhythm Type 1
  (Effects|Components|ParticleSystem|SetTemplate (Variables|Default|GetParticleSystem) (Utilities|Select :Index _type :NewEnumerator0 "/Game/MyMusicGame/Effects/FX_Cell_06.FX_Cell_06" :NewEnumerator1 "/Game/MagicEffects/UETools/MagicEffects/Effects/FX_Cell_03.FX_Cell_03"))
  (if (Utilities|Enum|Equal(Enum) _type "NewEnumerator1")
    (Utilities|Time|SetTimerbyFunctionName 0 "CheckPress" 0.02 true)))

(fn ConstructionScript)

(fn CheckPress
  (bind _time (Variables|Default|GetTime))
  (bind _playerref (Variables|Default|GetPlayerREF))
  (bind _curtime (Variables|/Game/MyMusicGame/Blueprints/GameMode/GamePawn.GamePawn_C|GetCurTime _playerref))
  (bind _returnvalue (Math|Float|Truncate _curtime))
  (bind _returnvalue_2 (- _returnvalue _time))
  (if (and (<= _returnvalue_2 200) (>= _returnvalue_2 -1))
    (if (Utilities|Array|Get(acopy) (Variables|/Game/MyMusicGame/Blueprints/GameMode/GamePawn.GamePawn_C|GetHolePressing (.AsGame%20Pawn (Utilities|Casting|CastToGamePawn (Game|Player|GetPlayerPawn 0)))) (Variables|Default|GetPosition))
      (Default|TypeEffect (Utilities|Array|Get(acopy) (Variables|/Game/MyMusicGame/Blueprints/GameMode/GamePawn.GamePawn_C|GetHoleCollection (Variables|Default|GetPlayerREF)) (Variables|Default|GetPosition)) false)
      (CallFunction|EventSuccessfulTyped))))

(fn CanbeTyped
  (bind _time (Variables|Default|GetTime))
  (bind _playerref (Variables|Default|GetPlayerREF))
  (bind _curtime (Variables|/Game/MyMusicGame/Blueprints/GameMode/GamePawn.GamePawn_C|GetCurTime _playerref))
  (bind _returnvalue (Math|Float|Truncate _curtime))
  (bind _returnvalue_2 (- _returnvalue _time))
  (bind _returnvalue_3 (Math|Integer|Absolute(Integer) _returnvalue_2))
  (if (<= _returnvalue_3 70)
    (return true true)
    (elif (<= _returnvalue_3 300)
      (return true false)
      (else
        (return false false)))))
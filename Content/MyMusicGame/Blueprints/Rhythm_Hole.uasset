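; Rhythm_Hole is a touchable hole actor for the music game that relays input to the player's GamePawn.
; Touch begin on its Box calls Typed on the pawn, while touch enter and leave set the hole's pressed state there.
; Its TypeEffect event spawns a particle emitter at the hole's location, tinted yellow when the IsCharaming flag is set.
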(event OnInputTouchBegin(Box)
  (params (FingerIndex :type ETouchIndex%20Enum :default "Touch1") (TouchedComponent :type Primitive%20Component%20Object%20Reference))
  ;[1 1 1] Touch Gestures
  (bind _asgame_pawn (Utilities|Casting|CastToGamePawn (Game|Player|GetPlayerPawn 0)))
  (Default|Typed _asgame_pawn self))

(event OnInputTouchLeave(Box)
  (params (FingerIndex :type ETouchIndex%20Enum :default "Touch1") (TouchedComponent :type Primitive%20Component%20Object%20Reference))
  ;[1 1 1] Touch Gestures
  (bind _asgame_pawn (Utilities|Casting|CastToGamePawn (Game|Player|GetPlayerPawn 0)))
  (Default|SetHolePressState _asgame_pawn self false))

(event OnInputTouchEnter(Box)
  (params (FingerIndex :type ETouchIndex%20Enum :default "Touch1") (TouchedComponent :type Primitive%20Component%20Object%20Reference))
  ;[1 1 1] Touch Gestures
  (bind _asgame_pawn (Utilities|Casting|CastToGamePawn (Game|Player|GetPlayerPawn 0)))
  (Default|SetHolePressState _asgame_pawn self true))

(event Custom|TypeEffect
  (params (IsCharaming :type Boolean))
  (bind _returnvalue (Effects|SpawnEmitteratLocation "/Game/MyMusicGame/Effects/TypeEffect.TypeEffect" (Transformation|GetActorLocation)))
  (if IsCharaming
    (Effects|Components|ParticleSystem|SetColorParameter _returnvalue "Color" "(R=1.000000,G=1.000000,B=0.000000,A=1.000000)")))

(fn ConstructionScript)